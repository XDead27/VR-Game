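; OrbSpawner is a scene component on a pawn that periodically spawns teleport orbs at its own location.
; Tick feeds a two-second Delay, creating a repeating timer that spawns TeleportOrb_BP with the owning pawn as its teleport target, unless collision blocks it.
; Each new orb has mesh physics disabled and snaps onto the component, keeping world scale.
; Debug prints report the orb's location or a collision failure.
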(event EventBeginPlay)

(event EventTick
  (params (DeltaSeconds :type Float%20%28single-precision%29))
  (Utilities|FlowControl|Delay 2.0)
  (Utilities|FlowControl|Sequence
    (:then_0
      (bind _aspawn (Utilities|Casting|CastToPawn (Components|GetOwner self)))
      (bind _returnvalue (Game|SpawnActorfromClass "/Game/Blueprints/TeleportOrb_BP.TeleportOrb_BP_C" (Transformation|GetWorldTransform) "AdjustIfPossibleButDontSpawnIfColliding" 0 _aspawn 0))
      (if (Utilities|IsValid _returnvalue)
        (Physics|SetSimulatePhysics (Variables|/Script/CAAI.TeleportOrb|GetMesh _returnvalue) false)
        (Transformation|AttachComponentToComponent (Variables|/Script/Engine.Actor|GetRootComponent _returnvalue) self "None" "SnapToTarget" "SnapToTarget" "KeepWorld" true)
        (Development|PrintString (Utilities|String|ToString(Vector) (Transformation|GetActorLocation _returnvalue)))
        (else
          (Development|PrintString "colliding"))))))